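; BP_PaddlePawn_R is a Pong paddle pawn moved by the P1_MoveUp input axis.
; Both that axis event and an in-bounds Tick feed AddMovementInput along the control rotation's forward vector, scaled by the axis value.
; Each Tick also checks world X against hard-coded limits and snaps the paddle just inside when it overshoots, skipping that Tick's movement call.
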(event `self.ReceiveTick`
  (params (DeltaSeconds :type "Float (single-precision)"))
  ;[1 1 1] Boundry Stop
  (if (< (.x (`self.K2_GetActorLocation`)) -326.0)
    (`self.K2_SetActorLocation` (`KismetMathLibrary.MakeVector` -325.0 (.y (`self.K2_GetActorLocation`)) (.z (`self.K2_GetActorLocation`))))
    (elif (> (.x (`self.K2_GetActorLocation`)) 56.0)
      (`self.K2_SetActorLocation` (`KismetMathLibrary.MakeVector` 55.0 (.y (`self.K2_GetActorLocation`)) (.z (`self.K2_GetActorLocation`))))
      (else
        ;[1 1 1] Player paddle movement
        (`self.AddMovementInput` (`KismetMathLibrary.GetForwardVector` (`self.GetControlRotation`)) (stale `InputAxis|P1_MoveUp` AxisValue) :!label _label)))))

(event `InputAxis|P1_MoveUp`
  (params (AxisValue :type "Float (single-precision)"))
  ;[1 1 1] Player paddle movement
  (goto _label))

(fn `UserConstructionScript`)