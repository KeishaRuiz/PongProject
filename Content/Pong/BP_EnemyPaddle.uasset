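; BP_EnemyPaddle is the computer-controlled paddle in a Pong game, chasing the ball along the X axis.
; Every Tick it looks up all BP_Ball actors and nudges its physics Cube toward each with a clamped impulse based on the X offset.
; Outside fixed X limits, it instead snaps back just inside and zeroes velocity.
; An AIPaddleSpeed multiplier exists but is left unconnected, so it has no effect.
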(event `self.ReceiveTick`
  (params (DeltaSeconds :type "Float (single-precision)"))
  (bind _outactors (`GameplayStatics.GetAllActorsOfClass` "/Game/Pong/BP_Ball.BP_Ball_C"))
  (for _array_element _outactors
    (bind _asbp_ball (cast `/Game/Pong/BP_Ball` _array_element))
    (if (< (.x (`self.K2_GetActorLocation`)) -326.0)
      (`self.K2_SetActorLocation` (`KismetMathLibrary.MakeVector` -325.0 (.y (`self.K2_GetActorLocation`)) (.z (`self.K2_GetActorLocation`))))
      (`PrimitiveComponent.SetPhysicsLinearVelocity` (`self.Cube`) (0.0 0.0 0.0) false "None")
      (elif (> (.x (`self.K2_GetActorLocation`)) 56.0)
        (`self.K2_SetActorLocation` (`KismetMathLibrary.MakeVector` 55.0 (.y (`self.K2_GetActorLocation`)) (.z (`self.K2_GetActorLocation`))))
        (`PrimitiveComponent.SetPhysicsLinearVelocity` (`self.Cube`) (0.0 0.0 0.0) false "None")
        (else
          (`PrimitiveComponent.AddImpulse` (`self.Cube`) (`KismetMathLibrary.MakeVector` (`KismetMathLibrary.FClamp` (- (.x (`self.K2_GetActorLocation` _asbp_ball)) (.x (`self.K2_GetActorLocation`))) -10.0 10.0)) "None" false))))))

(fn `UserConstructionScript`)